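; Floor 1 manager stub for an objective chain of two levers, sigil fragments, a boss gate and an Ascension Gate, plus hub and floor travel.
; Lever and sigil functions call CheckBossGate, while OnBossDefeated handles the Ascension Gate.
; Logic is unfinished: setters write false or zero, gate branches are constant true with comparisons unconnected, and level loads target "None".
; BeginPlay is disabled, and duplicate node chains never run.
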(event EventBeginPlay)

(event Collision|EventActorBeginOverlap
  (params (OtherActor :type Actor%20Object%20Reference)))

(event EventTick
  (params (DeltaSeconds :type Float%20%28single-precision%29)))

(fn ConstructionScript)

(fn PullLeverA
  (Variables|Objectives|SetbLeverA_Pulled false)
  (Development|PrintString "[Floor1] Lever A pulled!")
  (CallFunction|CheckBossGate))

(fn PullLeverB
  (Variables|Objectives|SetbLeverB_Pulled false)
  (Development|PrintString "[Floor1] Lever B pulled!")
  (CallFunction|CheckBossGate))

(fn CollectSigil
  (Variables|Objectives|SetSigilCount 0)
  (Development|PrintString "[Floor1] Sigil fragment collected!")
  (CallFunction|CheckBossGate))

(fn CheckBossGate
  (if true
    (if true
      (Variables|Default|SetbBossGateOpen false)
      (Development|PrintString "[Floor1] BOSS GATE OPENS! The way forward is clear!")
      (else
        (Development|PrintString "[Floor1] Boss gate locked. Collect sigils and pull both levers.")))
    (else
      (Development|PrintString "[Floor1] Both levers must be pulled first."))))

(fn OnBossDefeated
  (Variables|Default|SetbBossDefeated false)
  (Variables|Objectives|SetbAscensionGateEnabled false)
  (Development|PrintString "[Floor1] BOSS DEFEATED! Ascension Gate unlocked!"))

(fn TraveltoFloor1
  (Development|PrintString "[Travel] Loading Map_Floor01_Ironcatacomb...")
  (Game|OpenLevel(byName) "None"))

(fn ReturntoHub
  (Development|PrintString "[Travel] Returning to Map_HubCitadelCity...")
  (Game|OpenLevel(byName) "None"))